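; Construction-script Blueprint that lays a chosen mesh along a spline as deforming spline mesh components with two material slots.
; The SplineMeshVar setting selects the layout: one segment per pair of spline points using their tangents, or segments at fixed Spacing along the spline's length.
; The spacing layout builds tangents from spline direction scaled by Spacing plus TangentScaleAdd.
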(fn ConstructionScript
  (|Wire))