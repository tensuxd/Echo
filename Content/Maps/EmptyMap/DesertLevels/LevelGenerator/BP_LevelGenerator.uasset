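; BP_LevelGenerator spawns randomly chosen, connected dungeon rooms when play begins.
; It places a BP_DungeonRoom1 start room at its own transform and collects the child components of that room's ExitsFolder as candidate exits.
; It then spawns one random room from RoomList at a random exit's transform and stores it as LatestRoom.
; The new room's exits are not collected, so generation stops after that single attachment.
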(event Custom|Spawn%20Start%20Room
  ;[0 1 0.09575 1 30] Spawn Start Room
  (bind _returnvalue (Game|SpawnActorfromClass "/Game/Maps/EmptyMap/DesertLevels/LevelGenerator/BP_DungeonRoom1.BP_DungeonRoom1_C" (Transformation|GetWorldTransform (Variables|Default|GetDefaultSceneRoot)) "AlwaysSpawn" "MultiplyWithRoot" 0 0))
  (Utilities|Array|AppendArray (Variables|Default|GetExits%20List) (Components|GetChildrenComponents (Variables|/Game/Maps/EmptyMap/DesertLevels/LevelGenerator/BP_MasterRoom.BP_MasterRoom_C|GetExitsFolder _returnvalue) false)))

(event Custom|Spawn%20Next%20Room
  (Variables|Default|SetSelected%20Exit%20Point (.OutItem (Utilities|Array|Random (Variables|Default|GetExits%20List))))
  (bind _returnvalue (Game|SpawnActorfromClass (.OutItem (Utilities|Array|Random (Variables|Default|GetRoom%20List))) (Transformation|GetWorldTransform (Variables|Default|GetSelected%20Exit%20Point)) "Undefined" "MultiplyWithRoot" 0 0))
  (bind _asbp_master_room (Utilities|Casting|CastToBP_MasterRoom _returnvalue))
  (Variables|Default|SetLatest%20Room _asbp_master_room))

(event EventBeginPlay
  (CallFunction|SpawnStartRoom)
  (CallFunction|SpawnNextRoom))

(fn ConstructionScript)