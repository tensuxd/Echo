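; BP_FootstepNotify is an animation notify that plays surface-dependent footstep sounds.
; It traces 100 units down from the mesh owner's location on the Visibility channel, leaving persistent debug lines.
; The hit's physical surface type selects a footstep sound cue, with concrete as the fallback; a miss plays nothing.
; Every sound plays at the world origin rather than the hit or actor location.
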(fn ReceivedNotify
  (params (MeshComp :type Skeletal%20Mesh%20Component%20Object%20Reference) (Animation :type Anim%20Sequence%20Base%20Object%20Reference) (EventReference :type Anim%20Notify%20Event%20Reference%20Structure%20%28by%20ref%29))
  (bind _returnvalue (Components|GetOwner MeshComp))
  (bind _returnvalue_2 (Transformation|GetActorLocation _returnvalue))
  (bind (_outhit _returnvalue_3) (Collision|LineTraceByChannel _returnvalue_2 (+ _returnvalue_2 (* (Transformation|GetActorUpVector _returnvalue) -1e+02)) "TraceTypeQuery1" false 0 "Persistent"))
  (if _returnvalue_3
    (switch Utilities|FlowControl|Switch|SwitchonEPhysicalSurface (Collision|GetSurfaceType _outhit)
      (:SurfaceType_Default
        (Audio|PlaySoundatLocation "/Game/System/Audio/Footesteps/Concrete/SC_ConcreteFootstep.SC_ConcreteFootstep" "0, 0, 0" "0, 0, 0" 1.0 1.0 0.0 0 0 0 0 :!label _label))
      (:SurfaceType1
        (Audio|PlaySoundatLocation "/Game/System/Audio/Footesteps/Wood/SC_WoodFootstep.SC_WoodFootstep" "0, 0, 0" "0, 0, 0" 1.0 1.0 0.0 0 0 0 0))
      (:SurfaceType2
        (Audio|PlaySoundatLocation "/Game/System/Audio/Footesteps/Steel/SC_SteelFootstep.SC_SteelFootstep" "0, 0, 0" "0, 0, 0" 1.0 1.0 0.0 0 0 0 0))
      (:SurfaceType3
        (Audio|PlaySoundatLocation "/Game/System/Audio/Footesteps/Forest/SC_ForestFootstep.SC_ForestFootstep" "0, 0, 0" "0, 0, 0" 1.0 1.0 0.0 0 0 0 0))
      (:SurfaceType4
        (Audio|PlaySoundatLocation "/Game/System/Audio/Footesteps/Snow/SC_SnowFootstep.SC_SnowFootstep" "0, 0, 0" "0, 0, 0" 1.0 1.0 0.0 0 0 0 0))
      (:SurfaceType5
        (Audio|PlaySoundatLocation "/Game/System/Audio/Footesteps/Bush/SC_BushFootstep.SC_BushFootstep" "0, 0, 0" "0, 0, 0" 1.0 1.0 0.0 0 0 0 0))
      (:SurfaceType6
        (goto _label))
      (:SurfaceType7
        (Audio|PlaySoundatLocation "/Game/System/Audio/Footesteps/Dirt/SC_DirtFootstep.SC_DirtFootstep" "0, 0, 0" "0, 0, 0" 1.0 1.0 0.0 0 0 0 0))
      (:SurfaceType8
        (Audio|PlaySoundatLocation "/Game/System/Audio/Footesteps/Garbage/SC_MusorFootstep.SC_MusorFootstep" "0, 0, 0" "0, 0, 0" 1.0 1.0 0.0 0 0 0 0)))
    (return false)))