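; Base interactable item actor that shows an interaction prompt and outline when the player character (BP_TempPerson) is near.
; Sphere overlap creates WBP_InteractHud in the widget component, plays its pop-up, applies an outline overlay material and enables CanPressE.
; Leaving reverses this and removes the widget after a short delay.
; CanResiveTrace toggles the same hint state from outside, and DestroyServer destroys the actor.
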(event OnComponentBeginOverlap(Sphere)
  (params (OverlappedComponent :type Primitive%20Component%20Object%20Reference) (OtherActor :type Actor%20Object%20Reference) (OtherComp :type Primitive%20Component%20Object%20Reference) (OtherBodyIndex :type Integer) (bFromSweep :type Boolean) (SweepResult :type Hit%20Result%20Structure%20%28by%20ref%29))
  ;[0.15 0.15 0.15 0.5] Crosshair on collision
  (Utilities|Casting|CastToBP_TempPerson OtherActor)
  (if (Variables|Default|GetCanInteract)
    (bind _returnvalue (UserInterface|CreateWidget "/Game/System/Widgets/UI/Interact/WBP_InteractHud.WBP_InteractHud_C"))
    (bind _output_get (Variables|Default|SetInteractWidget _returnvalue))
    (UserInterface|SetWidget (Variables|Default|GetWidget) _output_get)
    (Rendering|SetVisibility (Variables|Default|GetWidget) true false)
    (bind _interactwidget (Variables|Default|GetInteractWidget)
      (:then
        (if (not (Variables|Default|GetHintVisible))
          (UserInterface|Animation|PlayAnimation _interactwidget (Variables|/Game/System/Widgets/UI/Interact/WBP_InteractHud.WBP_InteractHud_C|GetPopUp _interactwidget) 0.0 1 "Forward" 1.5 false)
          (Variables|Default|SetHintVisible true)
          (Rendering|Material|SetOverlayMaterial (Variables|Default|GetStaticMesh) "/Game/System/Materials/OutlineMaterial/M_Outline.M_Outline" :!class /Script/Engine.MeshComponent)
          (Variables|Default|SetCanPressE true)))
      (:else))))

(event OnComponentEndOverlap(Sphere)
  (params (OverlappedComponent :type Primitive%20Component%20Object%20Reference) (OtherActor :type Actor%20Object%20Reference) (OtherComp :type Primitive%20Component%20Object%20Reference) (OtherBodyIndex :type Integer))
  (Utilities|Casting|CastToBP_TempPerson OtherActor)
  (if (Variables|Default|GetCanInteract)
    (bind _interactwidget (Variables|Default|GetInteractWidget)
      (:then
        (if (Variables|Default|GetHintVisible)
          (UserInterface|Animation|PlayAnimation _interactwidget (Variables|/Game/System/Widgets/UI/Interact/WBP_InteractHud.WBP_InteractHud_C|GetPopUp _interactwidget) 0.0 1 "Reverse" 1.5 false)
          (Variables|Default|SetHintVisible false)
          (Variables|Default|SetCanPressE false)
          (Rendering|Material|SetOverlayMaterial (Variables|Default|GetStaticMesh) 0 :!class /Script/Engine.MeshComponent))
        (Utilities|FlowControl|Delay 0.15)
        (Widget|RemovefromParent (Variables|Default|GetInteractWidget))
        (Variables|Default|SetInteractWidget 0)
        (Rendering|SetVisibility (Variables|Default|GetWidget) false false))
      (:else))))

(event Custom|DestroyServer
  (Actor|DestroyActor))

(event EventCanResiveTrace
  (params (CanInteract :type Boolean))
  (if (Variables|Default|GetCanInteract)
    (if CanInteract
      (bind _interactwidget (Variables|Default|GetInteractWidget)
        (:then
          (if (not (Variables|Default|GetHintVisible))
            (UserInterface|Animation|PlayAnimation _interactwidget (Variables|/Game/System/Widgets/UI/Interact/WBP_InteractHud.WBP_InteractHud_C|GetPopUp _interactwidget) 0.0 1 "Forward" 1.5 false)
            (Variables|Default|SetHintVisible true)
            (Rendering|Material|SetOverlayMaterial (Variables|Default|GetStaticMesh) "/Game/System/Materials/OutlineMaterial/M_Outline.M_Outline" :!class /Script/Engine.MeshComponent)
            (Variables|Default|SetCanPressE true)))
        (:else))
      (else
        (bind _interactwidget_2 (Variables|Default|GetInteractWidget)
          (:then
            (if (Variables|Default|GetHintVisible)
              (UserInterface|Animation|PlayAnimation _interactwidget_2 (Variables|/Game/System/Widgets/UI/Interact/WBP_InteractHud.WBP_InteractHud_C|GetPopUp _interactwidget_2) 0.0 1 "Reverse" 1.5 false)
              (Variables|Default|SetHintVisible false)
              (Rendering|Material|SetOverlayMaterial (Variables|Default|GetStaticMesh) 0 :!class /Script/Engine.MeshComponent)
              (Variables|Default|SetCanPressE false)))
          (:else))))))

(fn ConstructionScript)