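; Inventory component that gives the player a four-slot hotbar, shown through a WBP_InventoryBar widget created at BeginPlay.
; Mouse wheel with wrap-around and number keys move the highlighted slot, while G only clears the highlight.
; IsSlotFree both checks the current slot and stores the named item, taking its icon from ObjectTable.
; R drops the current item by spawning its table-defined actor at the player's location, then empties the slot.
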(event EventBeginPlay
  (bind _returnvalue (UserInterface|CreateWidget "/Game/System/Inventory/Widgets/WBP_InventoryBar.WBP_InventoryBar_C"))
  (bind _output_get (Variables|Default|SetInventoryBar _returnvalue))
  (UserInterface|Viewport|AddtoViewport _output_get 0)
  (Default|HightlightSlot (Variables|Default|GetInventoryBar) (Variables|Default|GetCurrentSlotIndex)))

(event Input|MouseEvents|MouseWheelUp
  (params (Key :type Key%20Structure :default "None"))
  (:Pressed
    (Default|UnhighlightSlot (Variables|Default|GetInventoryBar) (Variables|Default|GetCurrentSlotIndex))
    (bind _output_get (Variables|Default|SetCurrentSlotIndex (+ (Variables|Default|GetCurrentSlotIndex) 1)))
    (if (>= _output_get 4)
      (bind _output_get_2 (Variables|Default|SetCurrentSlotIndex 0))
      (Default|HightlightSlot (Variables|Default|GetInventoryBar) _output_get_2)
      (else
        (Default|HightlightSlot (Variables|Default|GetInventoryBar) (Variables|Default|GetCurrentSlotIndex))))))

(event Input|MouseEvents|MouseWheelDown
  (params (Key :type Key%20Structure :default "None"))
  (:Pressed
    (Default|UnhighlightSlot (Variables|Default|GetInventoryBar) (Variables|Default|GetCurrentSlotIndex))
    (bind _output_get (Variables|Default|SetCurrentSlotIndex (- (Variables|Default|GetCurrentSlotIndex) 1)))
    (if (<= _output_get -1)
      (bind _output_get_2 (Variables|Default|SetCurrentSlotIndex 3))
      (Default|HightlightSlot (Variables|Default|GetInventoryBar) _output_get_2)
      (else
        (Default|HightlightSlot (Variables|Default|GetInventoryBar) (Variables|Default|GetCurrentSlotIndex))))))

(event Input|KeyboardEvents|1
  (params (Key :type Key%20Structure :default "None"))
  (:Released
    (Default|UnhighlightSlot (Variables|Default|GetInventoryBar) (Variables|Default|GetCurrentSlotIndex))
    (bind _output_get (Variables|Default|SetCurrentSlotIndex 0))
    (Default|HightlightSlot (Variables|Default|GetInventoryBar) _output_get)))

(event Input|KeyboardEvents|2
  (params (Key :type Key%20Structure :default "None"))
  (:Released
    (Default|UnhighlightSlot (Variables|Default|GetInventoryBar) (Variables|Default|GetCurrentSlotIndex))
    (bind _output_get (Variables|Default|SetCurrentSlotIndex 1))
    (Default|HightlightSlot (Variables|Default|GetInventoryBar) _output_get)))

(event Input|KeyboardEvents|3
  (params (Key :type Key%20Structure :default "None"))
  (:Released
    (Default|UnhighlightSlot (Variables|Default|GetInventoryBar) (Variables|Default|GetCurrentSlotIndex))
    (bind _output_get (Variables|Default|SetCurrentSlotIndex 2))
    (Default|HightlightSlot (Variables|Default|GetInventoryBar) _output_get)))

(event Input|KeyboardEvents|4
  (params (Key :type Key%20Structure :default "None"))
  (:Released
    (Default|UnhighlightSlot (Variables|Default|GetInventoryBar) (Variables|Default|GetCurrentSlotIndex))
    (bind _output_get (Variables|Default|SetCurrentSlotIndex 3))
    (Default|HightlightSlot (Variables|Default|GetInventoryBar) _output_get)))

(event Input|KeyboardEvents|G
  (params (Key :type Key%20Structure :default "None"))
  (:Released
    (Default|UnhighlightSlot (Variables|Default|GetInventoryBar) (Variables|Default|GetCurrentSlotIndex))))

(event Input|KeyboardEvents|R
  (params (Key :type Key%20Structure :default "None"))
  (:Pressed
    (if (not (== (Utilities|Array|Get(acopy) (Variables|Default|GetInventorySlot) (Variables|Default|GetCurrentSlotIndex)) ""))
      (CallFunction|DropItem (Utilities|Array|Get(acopy) (Variables|Default|GetInventorySlot) (Variables|Default|GetCurrentSlotIndex))))))

(fn IsSlotFree?
  (params (Object%20Name :type Name))
  (if (== (Utilities|Array|Get(acopy) (Variables|Default|GetInventorySlot) (Variables|Default|GetCurrentSlotIndex)) "")
    (CallFunction|GetItemInfo Object%20Name (Variables|Default|GetCurrentSlotIndex))
    (return true)
    (else
      (return false))))

(fn GetItemInfo
  (params (Item%20Name :type Name) (Empty%20Element :type Integer))
  (bind _returnvalue (Utilities|GetDataTableRow (Variables|Default|GetObject%20Table) Item%20Name)
    (:then
      (Utilities|Array|SetArrayElem (Variables|Default|GetInventorySlot) Empty%20Element Item%20Name)
      (Default|SlotChanges (Variables|Default|GetInventoryBar) Empty%20Element (.ObjectIcon (Utilities|Struct|BreakS_ObjectTableStruct _returnvalue)) false))))

(fn DropItem
  (params (Object%20Name :type Name))
  (bind _returnvalue (Game|GetPlayerCharacter 0))
  (bind _returnvalue_2 (Utilities|GetDataTableRow (Variables|Default|GetObject%20Table) Object%20Name)
    (:then
      (bind _returnvalue_3 (Game|SpawnActorfromClass (.ActorBP (Utilities|Struct|BreakS_ObjectTableStruct _returnvalue_2)) (Math|Transform|MakeTransform (+ (Transformation|GetActorLocation _returnvalue) (* (Transformation|GetActorForwardVector _returnvalue) "")) "0, 0, 0" "1.000000,1.000000,1.000000") "Undefined" "MultiplyWithRoot" 0 0))
      (Utilities|IsValid _returnvalue_3
        (:Is%20Valid
          (Utilities|Array|SetArrayElem (Variables|Default|GetInventorySlot) (Variables|Default|GetCurrentSlotIndex) "")
          (Default|SlotChanges (Variables|Default|GetInventoryBar) (Variables|Default|GetCurrentSlotIndex) 0 true))))))