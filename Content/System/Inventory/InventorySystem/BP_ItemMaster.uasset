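; BP_ItemMaster is an item actor for the inventory system that makes itself the current interactable through a Sphere overlap.
; On begin overlap, if the other actor's AC_InventorySystem implements BPI_Interact, it enables player 0 input and stores itself in that component's BPItemMaster.
; End overlap disables input and clears that reference if it still points here, but looks up the component on itself, not the overlapping actor.
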(event OnComponentBeginOverlap(Sphere)
  (params (OverlappedComponent :type Primitive%20Component%20Object%20Reference) (OtherActor :type Actor%20Object%20Reference) (OtherComp :type Primitive%20Component%20Object%20Reference) (OtherBodyIndex :type Integer) (bFromSweep :type Boolean) (SweepResult :type Hit%20Result%20Structure%20%28by%20ref%29))
  (bind _returnvalue (Actor|GetComponentbyClass OtherActor "/Game/System/Inventory/InventorySystem/AC_InventorySystem.AC_InventorySystem_C"))
  (if (Utilities|DoesObjectImplementInterface _returnvalue "/Game/System/Inventory/Interact/Blueprint/Interface/BPI_Interact.BPI_Interact_C")
    (Input|EnableInput (Game|GetPlayerController 0))
    (Variables|/Game/System/Inventory/InventorySystem/AC_InventorySystem.AC_InventorySystem_C|SetBP_ItemMaster _returnvalue self)))

(event OnComponentEndOverlap(Sphere)
  (params (OverlappedComponent :type Primitive%20Component%20Object%20Reference) (OtherActor :type Actor%20Object%20Reference) (OtherComp :type Primitive%20Component%20Object%20Reference) (OtherBodyIndex :type Integer))
  (bind _returnvalue (Actor|GetComponentbyClass "/Game/System/Inventory/InventorySystem/AC_InventorySystem.AC_InventorySystem_C"))
  (if (Utilities|DoesObjectImplementInterface _returnvalue "/Game/System/Inventory/Interact/Blueprint/Interface/BPI_Interact.BPI_Interact_C")
    (if (== self (Variables|/Game/System/Inventory/InventorySystem/AC_InventorySystem.AC_InventorySystem_C|GetBP_ItemMaster _returnvalue))
      (Input|DisableInput (Game|GetPlayerController 0))
      (Variables|/Game/System/Inventory/InventorySystem/AC_InventorySystem.AC_InventorySystem_C|SetBP_ItemMaster _returnvalue 0))))

(fn ConstructionScript)