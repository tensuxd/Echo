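; Inventory actor component that tracks a selected slot for mouse-wheel cycling through inventory slots.
; MouseWheelUp and MouseWheelDown step SelectedSlot by one, stopping at MaxSlots and at zero without wrapping.
; PickUp and AddToInventory are empty stubs, and BeginPlay and Tick are unused.
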(event EventBeginPlay)

(event EventTick
  (params (DeltaSeconds :type Float%20%28single-precision%29)))

(fn PickUp)

(fn AddtoInventory)

(fn MouseWheelUp
  (if (not (== (Variables|Default|GetSelectedSlot) (Variables|Default|GetMaxSlots)))
    (Math|Integer|IncrementInt (Variables|Default|GetSelectedSlot))))

(fn MouseWheelDown
  (if (not (== (Variables|Default|GetSelectedSlot) 0))
    (Math|Integer|DecrementInt (Variables|Default|GetSelectedSlot))))