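; ShowWBLib is an actor Blueprint in the inventory slots system that provides a helper for showing or hiding a widget component for an interacting character.
; ShowWidgetFunc casts the other actor to Character; for a player, showing reveals the widget and enables input on this actor, while non-players instead become its owner.
; Hiding always hides the widget and disables input.
; The isPlayer macro accepts only locally controlled characters without an AI controller.
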(event EventBeginPlay)

(event Collision|EventActorBeginOverlap
  (params (OtherActor :type Actor%20Object%20Reference)))

(event EventTick
  (params (DeltaSeconds :type Float%20%28single-precision%29)))

(fn ConstructionScript)

(fn ShowWidgetFunc
  (params (WidgetTarget :type Widget%20Component%20Object%20Reference) (OtherActor :type Actor%20Object%20Reference) (IsShowingWidget :type Boolean))
  (bind _ascharacter (Utilities|Casting|CastToCharacter OtherActor))
  (if IsShowingWidget
    (bind _isnpc (Utilities|IsPlayer _ascharacter)
      (:true
        (Rendering|SetVisibility WidgetTarget true false)
        (Input|EnableInput (Game|GetPlayerController 0)))
      (:false
        _))
    (if (not _isnpc)
      (Actor|SetOwner _ascharacter)
      (return _ascharacter))
    (else
      (Rendering|SetVisibility WidgetTarget false false)
      (Input|DisableInput (Game|GetPlayerController 0))
      (return _ascharacter))))