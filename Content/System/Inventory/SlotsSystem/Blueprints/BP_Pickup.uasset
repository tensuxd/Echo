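; World pickup actor for the slot inventory system, letting a character collect an item with F.
; OnRep of ID resolves the item from DT_Inventory or a DropItem override, then sets the prompt text and skeletal mesh, falling back to static.
; Sphere overlap toggles the interact widget through a level ShowWBLib actor and caches the Character.
; F sends PickupItemMessage to that Character and, on success, destroys the pickup via DestroySERVER.
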(event OnComponentBeginOverlap(Sphere)
  (params (OverlappedComponent :type Primitive%20Component%20Object%20Reference) (OtherActor :type Actor%20Object%20Reference) (OtherComp :type Primitive%20Component%20Object%20Reference) (OtherBodyIndex :type Integer) (bFromSweep :type Boolean) (SweepResult :type Hit%20Result%20Structure%20%28by%20ref%29))
  ;[0.15 0.15 0.15 0.5] Vissible/Hidden interact widget
  (bind _outputcharacter (Default|ShowWidgetFunc (Variables|Default|GetAs%20Show%20WBLib) (Variables|Default|GetWidget) OtherActor true))
  (Variables|Default|SetCharacter _outputcharacter))

(event OnComponentEndOverlap(Sphere)
  (params (OverlappedComponent :type Primitive%20Component%20Object%20Reference) (OtherActor :type Actor%20Object%20Reference) (OtherComp :type Primitive%20Component%20Object%20Reference) (OtherBodyIndex :type Integer))
  ;[0.15 0.15 0.15 0.5] Vissible/Hidden interact widget
  (Default|ShowWidgetFunc (Variables|Default|GetAs%20Show%20WBLib) (Variables|Default|GetWidget) OtherActor false))

(event Custom|Update
  (bind _item (Variables|Default|GetItem))
  (bind (_displayname _pickupmesh _pickupmeshstatic) (Utilities|Struct|BreakST_Inventory_Item _item))
  (bind _aswbp_interact (Utilities|Casting|CastToWBP_Interact (UserInterface|GetWidget (Variables|Default|GetWidget))))
  (Rendering|Components|TextRender|SetText (Variables|/Game/System/Inventory/SlotsSystem/Widgets/WBP_Interact.WBP_Interact_C|GetTEXT _aswbp_interact) _displayname)
  (bind _returnvalue (Utilities|LoadAssetBlocking _pickupmesh))
  (bind _asskeletal_mesh (Utilities|Casting|CastToSkeletalMesh _returnvalue)
    (:then
      (Components|SkinnedMesh|SetSkinnedAssetandUpdate (Variables|Default|GetSkeletalMesh) _asskeletal_mesh true))
    (:CastFailed
      (bind _returnvalue_2 (Utilities|LoadAssetBlocking _pickupmeshstatic))
      (bind _asstatic_mesh (Utilities|Casting|CastToStaticMesh _returnvalue_2))
      (Components|StaticMesh|SetStaticMesh (Variables|Default|GetStaticMesh) _asstatic_mesh))))

(event EventBeginPlay
  (CallFunction|OnRepID)
  (bind _outactors (Actor|GetAllActorsOfClass "/Game/System/Inventory/SlotsSystem/Blueprints/ShowWBLib.ShowWBLib_C"))
  (bind _asshow_wblib (Utilities|Casting|CastToShowWBLib (Utilities|Array|Get(acopy) _outactors)))
  (Variables|Default|SetAs%20Show%20WBLib _asshow_wblib))

(event Input|KeyboardEvents|F
  (params (Key :type Key%20Structure :default "None"))
  (:Pressed
    (bind _success (Class|BPIInventory|PickupItem(Message) (Variables|Default|GetCharacter) (Variables|Default|GetID) (Variables|Default|GetItem)))
    (if _success
      (CallFunction|DestroySERVER))))

(event Custom|DestroySERVER
  ;[0.15 0.15 0.15 0.5] Destroy Server
  (Actor|DestroyActor))

(fn ConstructionScript
  (CallFunction|OnRepID))

(fn OnRepID
  (bind _returnvalue (Utilities|GetDataTableRow "/Game/System/Inventory/SlotsSystem/Data/DT_Inventory.DT_Inventory" (Variables|Default|GetID))
    (:then
      (Variables|Default|SetItem (select (!= (Utilities|Struct|BreakST_Inventory_Item (Variables|Default|GetDropItem)) "") (Variables|Default|GetDropItem) _returnvalue))
      (CallFunction|Update))))