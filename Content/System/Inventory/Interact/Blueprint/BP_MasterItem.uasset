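; BP_MasterItem is an interactable item actor in the inventory system, named as the master class for items.
; Interact prints a pickup message, calls DestroyServer, which chains to DestroyMulti to destroy the actor, then also calls DestroyActor directly.
; GetObjectName returns the item's ObjectName.
; No logic here adds the item to an inventory.
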(event Custom|DestroyServer
  (CallFunction|DestroyMulti))

(event Custom|DestroyMulti
  (Actor|DestroyActor))

(event EventInteract
  (params (Character :type BP%20Player%20Object%20Reference))
  (Utilities|IsValid self
    (:Is%20Valid
      (Development|PrintString "PickUp")
      (CallFunction|DestroyServer)
      (Actor|DestroyActor))))

(fn ConstructionScript)

(fn GetObjectName
  (return (Variables|Default|GetObjectName)))