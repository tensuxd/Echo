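; QuoteAngel is an interactable environment actor that shows or hides its widget when the player points at it from close range.
; A sphere overlap sets the proximity flag for BP_Player, while any actor ending overlap clears it.
; When pointed at nearby, it passes the widget, player and CanUse state to a ShowWBLib actor found at BeginPlay.
; It always reports that interaction is possible.
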(event OnComponentBeginOverlap(Sphere)
  (params (OverlappedComponent :type Primitive%20Component%20Object%20Reference) (OtherActor :type Actor%20Object%20Reference) (OtherComp :type Primitive%20Component%20Object%20Reference) (OtherBodyIndex :type Integer) (bFromSweep :type Boolean) (SweepResult :type Hit%20Result%20Structure%20%28by%20ref%29))
  (Utilities|Casting|CastToBP_Player OtherActor)
  (Variables|Default|SetIsClose? true))

(event OnComponentEndOverlap(Sphere)
  (params (OverlappedComponent :type Primitive%20Component%20Object%20Reference) (OtherActor :type Actor%20Object%20Reference) (OtherComp :type Primitive%20Component%20Object%20Reference) (OtherBodyIndex :type Integer))
  (Variables|Default|SetIsClose? false))

(event EventBeginPlay
  (bind _outactors (Actor|GetAllActorsOfClass "/Game/System/Inventory/SlotsSystem/Blueprints/ShowWBLib.ShowWBLib_C"))
  (bind _asshow_wblib (Utilities|Casting|CastToShowWBLib (Utilities|Array|Get(acopy) _outactors)))
  (Variables|Default|SetAs%20Show%20WBLib _asshow_wblib))

(event EventIsPointed
  (params (CanUse? :type Boolean) (PlayerBP :type BP%20Player%20Object%20Reference))
  (if (Variables|Default|GetIsClose?)
    (Default|ShowWidgetFunc (Variables|Default|GetAs%20Show%20WBLib) (Variables|Default|GetWidget) PlayerBP CanUse?)))

(fn ConstructionScript)

(fn PossibletoInteract
  (return true))