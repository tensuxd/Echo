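; Test AI pawn that wanders at random and gets distracted by perceived stimuli.
; Patrol sets a looping timer that moves it to a random reachable point near its current location, restarting on each successful arrival.
; A sensed AIPerception stimulus pauses that timer and sends the pawn to the stimulus location.
; After reaching it and waiting briefly, patrol resumes; failed moves have no handling.
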(event OnTargetPerceptionUpdated(AIPerception)
  (params (Actor :type Actor%20Object%20Reference) (Stimulus :type AI%20Stimulus%20Structure))
  (bind (_age _expirationage _strength _stimuluslocation _receiverlocation _tag _bsuccessfullysensed) (Utilities|Struct|BreakAIStimulus Stimulus))
  (if _bsuccessfullysensed
    (Utilities|Time|PauseTimerbyHandle (Variables|Default|GetPatrol%20Timer))
    (AI|AIMoveTo self _stimuluslocation 0 5.0 false
      (:OnSuccess
        (Utilities|FlowControl|Delay 2.0)
        (Utilities|Time|UnpauseTimerbyHandle (Variables|Default|GetPatrol%20Timer))
        (CallFunction|Patrol)))))

(event Custom|Patrol
  (bind _returnvalue (Utilities|Time|SetTimerbyEvent (delegate Custom|Start) 2.0 true))
  (Variables|Default|SetPatrol%20Timer _returnvalue))

(event Custom|Start
  (AI|AIMoveTo self (.RandomLocation (AI|Navigation|GetRandomReachablePointinRadius (Transformation|GetActorLocation) 5e+02 0 0)) 0 5.0 false
    (:OnSuccess
      (CallFunction|Patrol))))

(event EventBeginPlay
  (CallFunction|Patrol))

(fn ConstructionScript)